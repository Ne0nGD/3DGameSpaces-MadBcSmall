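; Moving laser hazard that travels along two relative control points and damages the first-person character it hits.
; The construction script sets the InterpToMovement path and duration, and BeginPlay colors the Niagara beam and impact by active state.
; While active, Tick line-traces forward to set the beam end and impact effect, damaging a living character every frame.
; Deactivate only clears the active flag, stopping trace updates and damage.
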(event Custom|Deactivate
  (Variables|Default|SetIsactive false))

(event EventTick
  (params (DeltaSeconds :type Float%20%28single-precision%29))
  (bind _returnvalue (Transformation|GetActorLocation))
  (bind _returnvalue_2 (Transformation|GetActorForwardVector))
  (bind _distance (Variables|Damage|GetDistance))
  (bind _niagara_laserimpact (Variables|Default|GetNiagara%20LaserImpact))
  (bind _returnvalue_3 (* _returnvalue_2 _distance))
  (bind _returnvalue_4 (+ _returnvalue _returnvalue_3))
  (Variables|Default|SetTraceEnd _returnvalue_4)
  (if (Variables|Default|GetIsactive)
    (bind _outhit (Collision|LineTraceByChannel _returnvalue _returnvalue_4 "TraceTypeQuery2" false 0 (Variables|Debug|GetDraw%20Debug%20Type)))
    (Variables|Default|SetHit (.bblockinghit _outhit))
    (Variables|Default|SetHitLocation (.location _outhit))
    (Effects|Components|ParticleSystem|SetVectorParameter (Variables|Default|GetNiagara%20Laser) "LaserEnd" (select (Variables|Default|GetHit) (Variables|Default|GetHitLocation) (Variables|Default|GetTraceEnd)))
    (Rendering|SetVisibility _niagara_laserimpact (Variables|Default|GetHit) false)
    (Transformation|SetWorldLocation _niagara_laserimpact (Variables|Default|GetHitLocation) false false)
    (bind _asfirst_person_character (Utilities|Casting|CastToFirstPersonCharacter (.hitactor _outhit)))
    (if (not (Variables|/Game/David/FirstPersonCharacter/FirstPersonCharacter.FirstPersonCharacter_C|GetIsDead _asfirst_person_character))
      (Game|Damage|ApplyDamage _asfirst_person_character (Variables|Damage|GetBase%20Damage) 0 0))))

(event EventBeginPlay
  (if (Variables|Default|GetIsactive)
    (Effects|Components|ParticleSystem|SetColorParameter (Variables|Default|GetNiagara%20Laser) "Color" "(R=194.929413,G=0.000000,B=255.000000,A=1.000000)")
    (Effects|Components|ParticleSystem|SetColorParameter (Variables|Default|GetNiagara%20LaserImpact) "Color" "(R=0.918059,G=0.000000,B=1.000000,A=1.000000)")
    (else
      (Effects|Components|ParticleSystem|SetColorParameter (Variables|Default|GetNiagara%20Laser) "Color" "(R=255.000000,G=0.000000,B=0.007296,A=0.000000)")
      (Effects|Components|ParticleSystem|SetColorParameter (Variables|Default|GetNiagara%20LaserImpact) "Color" "(R=1.000000,G=0.000000,B=0.007402,A=0.000000)"))))

(fn ConstructionScript
  (bind _interptomovement (Variables|Default|GetInterpToMovement))
  (Variables|/Script/Engine.InterpToMovementComponent|SetControlPoints _interptomovement (Utilities|Array|MakeArray (Utilities|Struct|MakeInterpControlPoint (Variables|Default|GetLocation) true) (Utilities|Struct|MakeInterpControlPoint (Variables|Default|GetLocation2) true)))
  (Variables|/Script/Engine.InterpToMovementComponent|SetDuration _interptomovement (Variables|Default|GetDuration)))